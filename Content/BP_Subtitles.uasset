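; Subtitle display actor that shows captions through a SubtitlesFrontend widget mounted with a spring arm.
; On BeginPlay it loads the subtitle settings, hiding itself when they are off or applying the text size otherwise.
; New lines are filtered by Voice in On mode and passed whole in Closed Captions mode.
; ChangeArmSpring switches between a short rigid arm and a longer lagged arm with collision testing.
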(event Custom|CustomEvent
  (params (subtitles :type Array%20of%20Advanced%20Subtitle%20Cue%20Structures)))

(event EventBeginPlay
  (bind _subtitlesettings (CallFunction|GetSubtitleSettings))
  (CallFunction|LoadSettings _subtitlesettings))

(event EventPushSubtitles
  (params (subtitles :type Array%20of%20Advanced%20Subtitle%20Cue%20Structures))
  (CallFunction|AddSubtitles subtitles))

(event EventChangeArmSpring
  (params (enable :type Boolean))
  (bind _springarm (Variables|Default|GetSpringArm))
  (bind _output_get (Variables|/Script/Engine.SpringArmComponent|SetbDoCollisionTest _springarm (not enable)))
  (bind _output_get_2 (Variables|/Script/Engine.SpringArmComponent|SetbEnableCameraLag _springarm _output_get))
  (if _output_get_2
    (Variables|/Script/Engine.SpringArmComponent|SetTargetArmLength _springarm 75.0)
    (else
      (Variables|/Script/Engine.SpringArmComponent|SetTargetArmLength _springarm 4e+01))))

(fn ConstructionScript)

(fn LoadSettings
  (params (Subtitle%20Settings :type Subtitles%20Settings%20Structure))
  (bind _output_get (Variables|Default|SetSubtitle%20Settings Subtitle%20Settings))
  (switch Utilities|FlowControl|Switch|SwitchonESubtitleModes (.SubtitleMode (Utilities|Struct|BreakSubtitlesSettings _output_get))
    (:NewEnumerator0
      (Rendering|SetActorHiddenInGame true))
    (:NewEnumerator1
      (Rendering|SetActorHiddenInGame false :!label _label)
      (Class|SubtitleFrontendInterface|SetSubtitleOffsetSize(Message) (UserInterface|GetWidget (Variables|Default|GetSubtitlesFrontend)) (.SubtitleSize (Utilities|Struct|BreakSubtitlesSettings _output_get)))
      (return))
    (:NewEnumerator2
      (goto _label))))

(fn AddSubtitles
  (params (NewParam :type Array%20of%20Advanced%20Subtitle%20Cue%20Structures))
  (bind _newlocalvar_0 (LocalVariables|GetNewLocalVar_0))
  (switch Utilities|FlowControl|Switch|SwitchonESubtitleModes (.SubtitleMode (Utilities|Struct|BreakSubtitlesSettings (Variables|Default|GetSubtitle%20Settings)))
    (:NewEnumerator1
      (for _array_element NewParam
        (if (== (.Voice (Utilities|Struct|BreakAdvancedSubtitleCue _array_element)) 0)
          (Utilities|Array|Add _newlocalvar_0 _array_element)))
      (Class|Subtitles|PushSubtitles _newlocalvar_0))
    (:NewEnumerator2
      (Class|Subtitles|PushSubtitles NewParam))))